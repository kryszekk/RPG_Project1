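; Base pickup actor that players can highlight and interact with through its InteractableComponent.
; On BeginPlay it hands its static mesh to that component for highlighting.
; When it exists as a child actor, such as an equipped weapon, it switches the mesh to WorldDynamic so interaction traces ignore it.
; DestroyAnActor clears tags, hides the mesh and delays destruction to avoid pending-kill access errors.
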(event EventBeginPlay
  (|CallParentFunction)
  ;[1 1 1] For highlight
  (Variables|/Game/_main/BP-Folder/BPs_Base/InteractableComponent.InteractableComponent_C|SetPrimitiveComponent (Variables|Default|GetInteractableComponent) (Variables|Default|GetStaticMesh))
  ;[1 1 1] Fix highlighting equipped weapons
  ;;[1 1 1] is attatched to a player as a child?
  (if (Class|Actor|IsChildActor)
    ;;[0.4993 1 0.4736] Sollution 1:  I can just change Collision type so Players "trace for interractable" nodes will not catch it
    (Collision|SetCollisionObjectType (Variables|Default|GetStaticMesh) "ECC_WorldDynamic")))

(event Collision|EventActorBeginOverlap
  (params (OtherActor :type Actor%20Object%20Reference))
  (|CallParentFunction OtherActor) ; This node is disabled and will not be called.\nDrag off pins to build functionality.
)

(event EventTick
  (params (DeltaSeconds :type Float%20%28single-precision%29))
  (|CallParentFunction DeltaSeconds) ; This node is disabled and will not be called.\nDrag off pins to build functionality.
)

(event EventDestroyAnActor
  ;[1 1 1] This is just to avoid an error (node tries to access Pending Kill Actor) - I can delete this nodes but errors will appear
  (Utilities|Array|Clear (Variables|Actor|GetTags))
  (Rendering|SetVisibility (Variables|Default|GetStaticMesh) false false)
  (Utilities|FlowControl|Delay 2.0)
  (Actor|DestroyActor self))

(fn ConstructionScript
  (|CallParentFunction))