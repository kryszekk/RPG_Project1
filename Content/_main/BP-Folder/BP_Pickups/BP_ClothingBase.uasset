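; Base clothing pickup that holds an apparel info struct and derives its stats procedurally.
; Unless CustomStats is set, the construction script rebuilds the struct, scaling armour, magic resistance and price from required level, quality and apparel-type multipliers.
; Weight depends only on apparel type.
; A ClothingInfo function returns the struct and amount; the event graph holds only disabled stubs.
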(event EventBeginPlay
  (|CallParentFunction) ; This node is disabled and will not be called.\nDrag off pins to build functionality.
)

(event Collision|EventActorBeginOverlap
  (params (OtherActor :type Actor%20Object%20Reference))
  (|CallParentFunction OtherActor) ; This node is disabled and will not be called.\nDrag off pins to build functionality.
)

(event EventTick
  (params (DeltaSeconds :type Float%20%28single-precision%29))
  (|CallParentFunction DeltaSeconds) ; This node is disabled and will not be called.\nDrag off pins to build functionality.
)

(fn ConstructionScript
  (|CallParentFunction)
  (CallFunction|ProceduralySetArmour))

(fn ProceduralySetArmour
  (if (not (.customstats (Variables|Default|GetS_ClothingInfo)))
    (switch Utilities|FlowControl|Switch|SwitchonE_ItemQuality (.itemquality (Variables|Default|GetS_ClothingInfo))
      (:NewEnumerator0
        (LocalVariables|SetQualityMultiplier 0.6))
      (:NewEnumerator1
        (LocalVariables|SetQualityMultiplier 0.8))
      (:NewEnumerator2
        (LocalVariables|SetQualityMultiplier 1.0))
      (:NewEnumerator3
        (LocalVariables|SetQualityMultiplier 1.2))
      (:NewEnumerator4
        (LocalVariables|SetQualityMultiplier 1.4))
      (:NewEnumerator5
        (LocalVariables|SetQualityMultiplier 1.6))
      (:NewEnumerator6
        (LocalVariables|SetQualityMultiplier 2.0)))
    (switch Utilities|FlowControl|Switch|SwitchonE_ApparelType (.appareltype (Variables|Default|GetS_ClothingInfo))
      (:NewEnumerator0
        (LocalVariables|SetApparelTypeMultiplier 0.5))
      (:NewEnumerator1
        (LocalVariables|SetApparelTypeMultiplier 0.1))
      (:NewEnumerator2
        (LocalVariables|SetApparelTypeMultiplier 0.1))
      (:NewEnumerator3
        (LocalVariables|SetApparelTypeMultiplier 0.3)))
    (Variables|Default|SetS_ClothingInfo (Utilities|Struct|MakeS_ClothingInfo (.name (Variables|Default|GetS_ClothingInfo)) (* (LocalVariables|GetApparelTypeMultiplier) 1e+01) (.icon (Variables|Default|GetS_ClothingInfo)) (.customstats (Variables|Default|GetS_ClothingInfo)) (* (* (* (.lvrequired (Variables|Default|GetS_ClothingInfo)) 5.0) (LocalVariables|GetQualityMultiplier)) (LocalVariables|GetApparelTypeMultiplier)) (* (* (* (.lvrequired (Variables|Default|GetS_ClothingInfo)) 5.0) (LocalVariables|GetQualityMultiplier)) (LocalVariables|GetApparelTypeMultiplier)) (.itemquality (Variables|Default|GetS_ClothingInfo)) (.appareltype (Variables|Default|GetS_ClothingInfo)) (* (Math|Float|Round (* (* (* (.lvrequired (Variables|Default|GetS_ClothingInfo)) 5.0) (LocalVariables|GetQualityMultiplier)) (LocalVariables|GetApparelTypeMultiplier))) 18) (.lvrequired (Variables|Default|GetS_ClothingInfo))))))

(fn ClothingInfo
  (return (Variables|Default|GetS_ClothingInfo) (Variables|Default|Getammount)))