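; Base Blueprint for junk pickups, holding an item info struct (name, weight, icon, use type, class reference) and an amount.
; The construction script rebuilds the struct with the actor's own class as the class reference, so each child class fills it in automatically.
; A JunkInfo function returns the struct and amount, while the event graph only passes BeginPlay to the parent.
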(event EventBeginPlay
  (|CallParentFunction))

(event Collision|EventActorBeginOverlap
  (params (OtherActor :type Actor%20Object%20Reference))
  (|CallParentFunction OtherActor) ; This node is disabled and will not be called.\nDrag off pins to build functionality.
)

(event EventTick
  (params (DeltaSeconds :type Float%20%28single-precision%29))
  (|CallParentFunction DeltaSeconds) ; This node is disabled and will not be called.\nDrag off pins to build functionality.
)

(fn ConstructionScript
  (|CallParentFunction)
  ;[1 1 1] Auto Set Class Reference
  (Variables|Default|SetS_JunkInfo (Utilities|Struct|MakeS_JunkInfo (.Name (Utilities|Struct|BreakS_JunkInfo (Variables|Default|GetS_JunkInfo))) (.Weight (Utilities|Struct|BreakS_JunkInfo (Variables|Default|GetS_JunkInfo))) (.Icon (Utilities|Struct|BreakS_JunkInfo (Variables|Default|GetS_JunkInfo))) (.UseType (Utilities|Struct|BreakS_JunkInfo (Variables|Default|GetS_JunkInfo))) (Utilities|GetClass self))))

(fn JunkInfo
  (return (Variables|Default|GetS_JunkInfo) (Variables|Default|Getammount)))