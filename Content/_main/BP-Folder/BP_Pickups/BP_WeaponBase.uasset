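; Base weapon pickup Blueprint that holds a weapon's stat struct and amount, exposed to other code through getters and a setter.
; Its construction script stamps the actor's class into the struct, then runs ProceduralySetDamage, which skips weapons flagged CustomStats.
; That function derives a damage budget from required level, quality and weapon type, randomly splitting it between physical and magical damage.
; Price scales with that budget, while weight depends only on weapon type.
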(event EventBeginPlay
  (|CallParentFunction))

(event Collision|EventActorBeginOverlap
  (params (OtherActor :type Actor%20Object%20Reference))
  (|CallParentFunction OtherActor) ; This node is disabled and will not be called.\nDrag off pins to build functionality.
)

(event EventTick
  (params (DeltaSeconds :type Float%20%28single-precision%29))
  (|CallParentFunction DeltaSeconds) ; This node is disabled and will not be called.\nDrag off pins to build functionality.
)

(event EventSetWeaponStats
  (params (S_WeaponInfo :type S%20Weapon%20Info%20Structure) (amount :type Integer))
  (Variables|Default|SetS_WeaponInfo S_WeaponInfo)
  (Variables|Default|SetAmount amount))

(fn ConstructionScript
  (|CallParentFunction)
  (Variables|Default|SetS_WeaponInfo (Utilities|Struct|MakeS_WeaponInfo (Utilities|GetClass self) (.Name (Utilities|Struct|BreakS_WeaponInfo (Variables|Default|GetS_WeaponInfo))) (.Weight (Utilities|Struct|BreakS_WeaponInfo (Variables|Default|GetS_WeaponInfo))) (.Icon (Utilities|Struct|BreakS_WeaponInfo (Variables|Default|GetS_WeaponInfo))) (.DamagePhysical (Utilities|Struct|BreakS_WeaponInfo (Variables|Default|GetS_WeaponInfo))) 0.0 (.WeaponType (Utilities|Struct|BreakS_WeaponInfo (Variables|Default|GetS_WeaponInfo))) (.lvRequired (Utilities|Struct|BreakS_WeaponInfo (Variables|Default|GetS_WeaponInfo))) (.Quality (Utilities|Struct|BreakS_WeaponInfo (Variables|Default|GetS_WeaponInfo))) (.CustomStats (Utilities|Struct|BreakS_WeaponInfo (Variables|Default|GetS_WeaponInfo))) (.Price (Utilities|Struct|BreakS_WeaponInfo (Variables|Default|GetS_WeaponInfo)))))
  (CallFunction|ProceduralySetDamage))

(fn ProceduralySetDamage
  (if (not (.customstats (Variables|Default|GetS_WeaponInfo)))
    ;[1 1 1] Set's procedural Damage ammount based on:
    ; -Level Required
    ; -WeaponQuality
    ; -WeaponType
    (switch Utilities|FlowControl|Switch|SwitchonE_ItemQuality (.quality (Variables|Default|GetS_WeaponInfo))
      (:NewEnumerator0
        (LocalVariables|SetqualityMultiplier 0.6))
      (:NewEnumerator1
        (LocalVariables|SetqualityMultiplier 0.8))
      (:NewEnumerator2
        (LocalVariables|SetqualityMultiplier 1.0))
      (:NewEnumerator3
        (LocalVariables|SetqualityMultiplier 1.2))
      (:NewEnumerator4
        (LocalVariables|SetqualityMultiplier 1.4))
      (:NewEnumerator5
        (LocalVariables|SetqualityMultiplier 1.6))
      (:NewEnumerator6
        (LocalVariables|SetqualityMultiplier 2.0)))
    (switch Utilities|FlowControl|Switch|SwitchonEWeaponType_E (.weapontype (Variables|Default|GetS_WeaponInfo))
      (:OneHanded
        (LocalVariables|SetweaponTypeMultiplier 0.9))
      (:TwoHanded
        (LocalVariables|SetweaponTypeMultiplier 1.2))
      (:Spears
        (LocalVariables|SetweaponTypeMultiplier 1.0))
      (:Gauntlets
        (LocalVariables|SetweaponTypeMultiplier 0.7)))
    (Variables|Default|SetS_WeaponInfo (Utilities|Struct|MakeS_WeaponInfo (.classreference (Variables|Default|GetS_WeaponInfo)) (.name (Variables|Default|GetS_WeaponInfo)) (* (LocalVariables|GetweaponTypeMultiplier) 3.0) (.icon (Variables|Default|GetS_WeaponInfo)) (Math|Conversions|ToFloat(Integer) (Math|Float|Round (- (* (* (* (.lvrequired (Variables|Default|GetS_WeaponInfo)) 5.0) (LocalVariables|GetqualityMultiplier)) (LocalVariables|GetweaponTypeMultiplier)) (/ (* (* (* (.lvrequired (Variables|Default|GetS_WeaponInfo)) 5.0) (LocalVariables|GetqualityMultiplier)) (LocalVariables|GetweaponTypeMultiplier)) (Math|Random|RandomFloatinRange 1.0 (* (* (* (.lvrequired (Variables|Default|GetS_WeaponInfo)) 5.0) (LocalVariables|GetqualityMultiplier)) (LocalVariables|GetweaponTypeMultiplier))))))) (Math|Conversions|ToFloat(Integer) (Math|Float|Round (/ (* (* (* (.lvrequired (Variables|Default|GetS_WeaponInfo)) 5.0) (LocalVariables|GetqualityMultiplier)) (LocalVariables|GetweaponTypeMultiplier)) (Math|Random|RandomFloatinRange 1.0 (* (* (* (.lvrequired (Variables|Default|GetS_WeaponInfo)) 5.0) (LocalVariables|GetqualityMultiplier)) (LocalVariables|GetweaponTypeMultiplier)))))) (.weapontype (Variables|Default|GetS_WeaponInfo)) (.lvrequired (Variables|Default|GetS_WeaponInfo)) (.quality (Variables|Default|GetS_WeaponInfo)) false (* 6 (Math|Float|Round (* (* (* (.lvrequired (Variables|Default|GetS_WeaponInfo)) 5.0) (LocalVariables|GetqualityMultiplier)) (LocalVariables|GetweaponTypeMultiplier))))))
    (return)))

(fn GetInventoryStructType
  (return "NewEnumerator0"))

(fn GetWeaponStats
  (return (Variables|Default|GetS_WeaponInfo)))

(fn WeaponInfo
  (return (Variables|Default|GetS_WeaponInfo) (Variables|Default|GetAmount)))