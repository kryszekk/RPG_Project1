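; Base Blueprint for text note pickups, holding a note struct (text, name, price, read flag, use type) and an amount.
; The construction script rebuilds the struct to stamp the actor's own class into its class reference.
; A setter event overwrites the struct and amount, while getter functions return them and a fixed inventory struct type.
; It has no active overlap or tick logic of its own.
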(event EventBeginPlay
  (|CallParentFunction) ; This node is disabled and will not be called.\nDrag off pins to build functionality.
)

(event Collision|EventActorBeginOverlap
  (params (OtherActor :type Actor%20Object%20Reference))
  (|CallParentFunction OtherActor) ; This node is disabled and will not be called.\nDrag off pins to build functionality.
)

(event EventTick
  (params (DeltaSeconds :type Float%20%28single-precision%29))
  (|CallParentFunction DeltaSeconds) ; This node is disabled and will not be called.\nDrag off pins to build functionality.
)

(event EventSetTextNotesStats
  (params (S_textNotes :type S%20Text%20Notes%20Structure) (amount :type Integer))
  (Variables|Default|SetS_TextNotes S_textNotes)
  (Variables|Default|SetAmount amount))

(fn ConstructionScript
  (|CallParentFunction)
  (Variables|Default|SetS_TextNotes (Utilities|Struct|MakeS_TextNotes (.text (Variables|Default|GetS_TextNotes)) (.price (Variables|Default|GetS_TextNotes)) (.hasbenread (Variables|Default|GetS_TextNotes)) (.name (Variables|Default|GetS_TextNotes)) (.usetype (Variables|Default|GetS_TextNotes)) (Utilities|GetClass self))))

(fn GetInventoryStructType
  (return "NewEnumerator6"))

(fn TextNotesInfo
  (return (Variables|Default|GetS_TextNotes) (Variables|Default|GetAmount)))