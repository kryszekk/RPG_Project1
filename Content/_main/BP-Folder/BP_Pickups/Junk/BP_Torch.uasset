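; BP_Torch is a torch pickup with a point light that burns out after about 15 real minutes (5 in-game hours) of draining.
; A slow timeline, started and stopped by external calls, fires an event that notifies PlayerOwner and then destroys the actor after a short delay.
; PlayerOwner is cleared on drop so the burnout message targets only held torches.
; Helper events set light visibility and mesh collision type.
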(event EventBeginPlay
  (|CallParentFunction))

(event Collision|EventActorBeginOverlap
  (params (OtherActor :type Actor%20Object%20Reference))
  (|CallParentFunction OtherActor) ; This node is disabled and will not be called.\nDrag off pins to build functionality.
)

(event EventTick
  (params (DeltaSeconds :type Float%20%28single-precision%29))
  (|CallParentFunction DeltaSeconds) ; This node is disabled and will not be called.\nDrag off pins to build functionality.
)

(event EventSetVisibility
  (params (State :type Boolean))
  (Rendering|SetVisibility (Variables|Default|GetPointLight) State false))

(event EventSetCollisionObjectType
  (params (Type :type ECollisionChannel%20Enum :default "ECC_WorldStatic"))
  (Collision|SetCollisionObjectType (Variables|Default|GetStaticMesh) Type))

(event EventStartDrainingDurability
  (params (PlayerReference :type Actor%20Object%20Reference))
  (Variables|Default|SetPlayerOwner PlayerReference)
  (Timeline|SlowTImeline PlayFromStart ; Currently ticks every 900 secs(5 in-game hours)(15min of irl time)
    (:EventTrack%20-%20Tick
      (Class|BPIPlayer|TorchDurabilityTerminated(Message) (Variables|Default|GetPlayerOwner))
      (Utilities|FlowControl|Delay 0.2)
      (Actor|DestroyActor))))

(event EventStopDrainingDurability
  (Timeline|SlowTImeline Stop ; Currently ticks every 900 secs(5 in-game hours)(15min of irl time)
    (:EventTrack%20-%20Tick
      (Class|BPIPlayer|TorchDurabilityTerminated(Message) (Variables|Default|GetPlayerOwner))
      (Utilities|FlowControl|Delay 0.2)
      (Actor|DestroyActor))))

(event EventUnsetPlayerReference
  (Variables|Default|SetPlayerOwner 0))

(fn ConstructionScript
  (|CallParentFunction))