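; Game instance that owns saving, loading and deleting of named save slots, with a looping timer that autosaves every five minutes.
; SaveGame deletes an existing slot and writes a fresh BP_SaveGameObj, reusing the loaded one only if deletion fails.
; Player location and rotation are stored in a save struct and teleported back on load; the level name is a placeholder and is never restored.
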(event EventInit
  (Utilities|Time|SetTimerbyFunctionName 0 "AutoSave" 3e+02 true) ; AutoSave timer
)

(fn SetSPlayerSaveData
  (bind _asbp_player (Utilities|Casting|CastToBP_Player (Game|GetPlayerCharacter 0)))
  (Variables|/Game/_main/BP-Folder/GameSave/BP_SaveGameObj.BP_SaveGameObj_C|SetPlayerSaveData (Variables|Default|GetSaveGameObject) (Utilities|Struct|MakeS_PlayerSaveData (Transformation|GetActorLocation _asbp_player) "a" (Transformation|GetActorRotation _asbp_player))))

(fn LoadSPlayerData
  (bind _savegameobject (Variables|Default|GetSaveGameObject))
  (bind _playersavedata (Variables|/Game/_main/BP-Folder/GameSave/BP_SaveGameObj.BP_SaveGameObj_C|GetPlayerSaveData _savegameobject))
  (bind _asbp_player (Utilities|Casting|CastToBP_Player (Game|GetPlayerCharacter 0)))
  (bind _output_get (LocalVariables|SetPlayerRef _asbp_player))
  (Transformation|SetActorLocation _output_get (.transform _playersavedata) false true)
  (Transformation|SetActorRotation (LocalVariables|GetPlayerRef) (.rotation _playersavedata)))

(fn DeleteGameSave
  (params (SaveSlotName :type String))
  (SaveGame|DeleteGameinSlot SaveSlotName))

(fn SaveGame
  (params (SaveSlotName :type String))
  (bind _returnvalue (SaveGame|DoesSaveGameExist SaveSlotName))
  (if _returnvalue
    ;[1 1 1] If creating save game onject more optimal than casting this nodes are here to stay
    (bind _returnvalue_2 (SaveGame|DeleteGameinSlot SaveSlotName))
    (if _returnvalue_2
      (bind _returnvalue_3 (SaveGame|CreateSaveGameObject "/Game/_main/BP-Folder/GameSave/BP_SaveGameObj.BP_SaveGameObj_C"))
      (Variables|Default|SetSaveGameObject _returnvalue_3)
      ;[0.1961 0.4219 0.1494] Sets data into SaveGameObject
      ; Do all the save data functions here.
      ; Eg. SaveNPC_Data, Save LevelData, etc.
      (SetSaveGameData|SetSPlayerSaveData :!label _label)
      (bind _returnvalue_4 (SaveGame|SaveGametoSlot (Variables|Default|GetSaveGameObject) SaveSlotName))
      (else
        (bind _returnvalue_5 (SaveGame|LoadGamefromSlot SaveSlotName))
        (bind _asbp_save_game_obj (Utilities|Casting|CastToBP_SaveGameObj _returnvalue_5)
          (:then
            (Variables|Default|SetSaveGameObject _asbp_save_game_obj)
            (goto _label))
          (:CastFailed
            (Development|PrintString "ERROR: 
Cast Failed in: MyGameInstance 
SaveGame function" true true "(R=1.000000,G=0.000000,B=0.015278,A=1.000000)" 2e+01)))))
    (else
      (bind _returnvalue_6 (SaveGame|CreateSaveGameObject "/Game/_main/BP-Folder/GameSave/BP_SaveGameObj.BP_SaveGameObj_C"))
      (Variables|Default|SetSaveGameObject _returnvalue_6)
      (goto _label))))

(fn AutoSave
  (MainSave/LoadGame|SaveGame "AutoSave")
  (Development|PrintString "Did auto Save" true true "(R=0.000000,G=1.000000,B=0.261645,A=1.000000)" 5.0))

(fn LoadGame
  (params (SaveSlotName :type String))
  (bind _returnvalue (SaveGame|DoesSaveGameExist SaveSlotName))
  (if _returnvalue
    (bind _returnvalue_2 (SaveGame|LoadGamefromSlot SaveSlotName))
    (bind _asbp_save_game_obj (Utilities|Casting|CastToBP_SaveGameObj _returnvalue_2)) ; do soft reference!
    (Variables|Default|SetSaveGameObject _asbp_save_game_obj)
    ;[0.1961 0.4219 0.1494] Do all the Load Data functions here.
    ; Eg. LoadNPC_Data, Load LevelData, etc.
    (LoadSaveGameData|LoadSPlayerData)
    (else
      (Development|PrintString "ERROR 
Save Slot doesn't exist 
in: MyGameInstance, f. LoadGame " true true "(R=1.000000,G=0.000000,B=0.046707,A=1.000000)" 2e+01))))