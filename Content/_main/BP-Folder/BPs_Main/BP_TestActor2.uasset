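; Test actor for the PlayerAttributes_AC component that simulates a level-scaled player loadout.
; SimulateSetup feeds the component's rest multiplier into its damage and armour setters, with values derived from attribute Level.
; It sets a one-handed physical left-hand attack, a two-handed magical right-hand attack and mixed-weight armour split across four slots.
; The SimulateSetup call in the event graph is disconnected, so nothing runs it at play.
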(event EventBeginPlay
  ;[1 1 1] This actor is designed to test:
  ;  PlayerAttributes_AC
)

(event Collision|EventActorBeginOverlap
  (params (OtherActor :type Actor%20Object%20Reference)))

(event EventTick
  (params (DeltaSeconds :type Float%20%28single-precision%29)))

(fn ConstructionScript)

(fn SimulateSetup
  (bind _playerattributes_ac (Variables|Default|GetPlayerAttributes_AC))
  (bind _lightarmour (LocalVariables|GetLightArmour))
  (bind _pattributes (Variables|/Script/RPG_Project1.PlayerAttributes_AC|GetPAttributes _playerattributes_ac))
  (bind _level (Utilities|Struct|BreakPlayerAttributes_F _pattributes))
  (bind _returnvalue (* _level 2.5))
  (bind _returnvalue_2 (* _level 0.0))
  (bind _returnvalue_3 (* _level 5.0))
  (bind _returnvalue_4 (* _returnvalue 0.1))
  (bind _returnvalue_5 (* _returnvalue 0.5))
  (bind _returnvalue_6 (* _returnvalue 0.1))
  (bind _returnvalue_7 (* _returnvalue 0.3))
  (bind _returnvalue_8 (Class|PlayerAttributesAC|CalculateRestMultiplier _playerattributes_ac))
  (Class|PlayerAttributesAC|SetDamageLMB _playerattributes_ac _returnvalue_8 (LocalVariables|GetOneHanded) _returnvalue_3 _returnvalue_2)
  (Class|PlayerAttributesAC|SetDamageRMB _playerattributes_ac _returnvalue_8 (LocalVariables|GetTwoHanded) _returnvalue_2 _returnvalue_3)
  (Class|PlayerAttributesAC|SetWholeArmour _playerattributes_ac _returnvalue_8 _returnvalue_5 _returnvalue_5 (LocalVariables|GetMediumArmour) _returnvalue_6 _returnvalue_6 _lightarmour _returnvalue_7 _returnvalue_7 (LocalVariables|GetHeavyArmour) _returnvalue_4 _returnvalue_4 _lightarmour))