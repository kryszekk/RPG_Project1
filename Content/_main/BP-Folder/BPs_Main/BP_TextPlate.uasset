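; BP_TextPlate is an interactable plate actor that shows a configurable text message on two widget components.
; On BeginPlay it registers its static mesh with the interactable component and writes DisplayedText into both widgets through their chat text message function.
; StartDisplayingText and StopDisplayingText events toggle the visibility of both widgets, with no caller for them in this graph.
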(event EventBeginPlay
  (bind _displayedtext (Variables|Default|GetDisplayedText))
  ;[1 1 1] Interact system requirements
  (Variables|/Script/RPG_Project1.Interactable_AC|SetPrimitiveComponent (Variables|Default|GetInteractable_AC) (Variables|Default|GetStaticMesh))
  (Class|ChatWI|SetChatText(Message) (UserInterface|GetUserWidgetObject (Variables|Default|GetWidget1)) _displayedtext "Normal" 0 0.0)
  (Class|ChatWI|SetChatText(Message) (UserInterface|GetUserWidgetObject (Variables|Default|GetWidget)) _displayedtext "Normal" 0 0.0))

(event Collision|EventActorBeginOverlap
  (params (OtherActor :type Actor%20Object%20Reference)))

(event EventTick
  (params (DeltaSeconds :type Float%20%28single-precision%29)))

(event EventStartDisplayingText
  (Rendering|SetVisibility (Variables|Default|GetWidget1) true false)
  (Rendering|SetVisibility (Variables|Default|GetWidget) true false))

(event EventStopDisplayingText
  (Rendering|SetVisibility (Variables|Default|GetWidget1) false false)
  (Rendering|SetVisibility (Variables|Default|GetWidget) false false))

(fn ConstructionScript)