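; BP_HumanoidAI is a humanoid AI Blueprint that slowly updates an NPC's wealth and rest over game time.
; On BeginPlay it calls its parent, then starts a slow timeline whose event track is commented as ticking every four in-game hours.
; Each timeline tick raises the wealth state, lowers rest in the basic attributes component and recalculates stats, avoiding per-frame Tick logic.
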(event EventBeginPlay
  (bind _bpc_basicattributes (Variables|Default|GetBPC_BasicAttributes))
  (|CallParentFunction)
  (Timeline|Slow%20timeline PlayFromStart ; Currently ticks every 720 secs  which is 4h of in-game time
    (:EventTrack%20-%20Tick
      (Variables|Default|SetcurrentWealthState (+ (Variables|Default|GetcurrentWealthState) 2))
      (Variables|/Game/_main/BP-Folder/BPs_Main/BPC_BasicAttributes.BPC_BasicAttributes_C|SetrestLevel _bpc_basicattributes (- (Variables|/Game/_main/BP-Folder/BPs_Main/BPC_BasicAttributes.BPC_BasicAttributes_C|GetrestLevel _bpc_basicattributes) 20))
      (Default|RecalculateStats _bpc_basicattributes))))

(event Collision|EventActorBeginOverlap
  (params (OtherActor :type Actor%20Object%20Reference))
  (|CallParentFunction OtherActor) ; This node is disabled and will not be called.\nDrag off pins to build functionality.
)

(event EventTick
  (params (DeltaSeconds :type Float%20%28single-precision%29))
  (|CallParentFunction DeltaSeconds) ; This node is disabled and will not be called.\nDrag off pins to build functionality.
)

(fn ConstructionScript
  (|CallParentFunction))