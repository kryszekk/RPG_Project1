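; Character attributes component that holds HP/MP/SP, regen, weapon damage, experience and death for its owner.
; BeginPlay and RecalculateStats derive stats from level, attributes and a clamped rest multiplier, scaling both equipped weapons' damage by weapon skill.
; Hit functions pass damage to the target's GetHit, which applies it with a 10% floor and ragdolls at zero HP, using messages to reach the owner.
; GainExp cuts rewards from lower-level sources and handles level-ups.
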(event Custom|RecalculateStats
  ;[1 1 1] UpdateStats. Call after:
  ; -Level UP
  ; -Learning new  Attribute  level
  ; -Equiped weapon changes
  (bind _multiplier (CallFunction|CalculateRestMultiplier))
  (StatsSet|SetMaxHpMpSp _multiplier)
  (StatsSet|SetRegen _multiplier)
  (StatsSet|SetDamage _multiplier)
  (Class|BPIBasicAttributes|StartRegen(Message) (Components|GetOwner)))

(event EventBeginPlay
  (Utilities|FlowControl|DoOnce false
    (:Completed
      (bind _multiplier (CallFunction|CalculateRestMultiplier))
      (StatsSet|SetInitialHpMpSp _multiplier)
      (bind _multiplier_2 (CallFunction|CalculateRestMultiplier))
      (StatsSet|SetMaxHpMpSp _multiplier_2)
      (StatsSet|SetRegen _multiplier_2)
      (StatsSet|SetDamage _multiplier_2)
      (Class|BPIBasicAttributes|StartRegen(Message) (Components|GetOwner)))))

(event EventTick
  (params (DeltaSeconds :type Float%20%28single-precision%29)))

(event EventGetHit
  (params (PhysicalDamage :type Float%20%28double-precision%29) (MagicalDamage :type Float%20%28double-precision%29))
  (bind _returnvalue (Components|GetOwner))
  (CallFunction|ReceiveWeaponDamage PhysicalDamage MagicalDamage)
  ;[1 0 0.01504] TODO call StartRegen  event
  (Class|BPIBasicAttributes|StartRegen(Message) _returnvalue)
  ;[1 1 1] Check whether character should die
  (if (<= (Variables|Actor'sbasicstats|GetCurrentHp) 0.0)
    (CallFunction|TurnonRagDoll)
    ;[1 1 1] Turn's off - Cylinder collision of a dead body
    (bind _collision (Class|BPICharacterBase|GetCollisionCyllinder(Message) _returnvalue))
    (Collision|SetCollisionProfileName _collision "NoCollision" true :!class /Script/Engine.PrimitiveComponent)
    (Variables|Default|SetIsDead true)
    (Development|PrintString (Utilities|String|BuildString(Integer) (Utilities|GetDisplayName _returnvalue) "Has just died" 0) true true "(R=1.000000,G=0.597584,B=0.069704,A=1.000000)" 5.0)))

(fn RMBHitAnActor
  (params (EnemyTarget :type BPI%20Basic%20Attributes%20Interface))
  (Default|GetHit EnemyTarget (Variables|RMBOffenceStats|GetRMB_PhysicalDamage) (Variables|RMBOffenceStats|GetRMB_MagicalDamage)))

(fn LMBHitAnActor
  (params (EnemyTarget :type BPI%20Basic%20Attributes%20Interface))
  (Default|GetHit EnemyTarget (Variables|LMBOffenceStats|GetLMB_PhysicalDamage) (Variables|LMBOffenceStats|GetLMB_MagicalDamage)))

(fn GainExp
  (params (Quest%20or%20enemy%20Level :type Byte) (EXP%20To%20be%20gained :type Float%20%28double-precision%29))
  ;[1 1 1] Is the Player's lv greater than enemy's lv
  (if (> (Variables|Actor'sStats|GetActor's%20level) Quest%20or%20enemy%20Level)
    ;[1 1 1] How much greater is the player's lv than killed enemy's level
    (if (== (- (Variables|Actor'sStats|GetActor's%20level) 1) Quest%20or%20enemy%20Level) ; is greater by 1?
      (LocalVariables|SetExp%20Gain%20Rate 0.8)
      (elif (== (- (Variables|Actor'sStats|GetActor's%20level) 2) Quest%20or%20enemy%20Level) ; is greater by 2?
        (LocalVariables|SetExp%20Gain%20Rate 0.6)
        (elif (== (- (Variables|Actor'sStats|GetActor's%20level) 3) Quest%20or%20enemy%20Level) ; is greater by 3?
          (LocalVariables|SetExp%20Gain%20Rate 0.4)
          (elif (== (- (Variables|Actor'sStats|GetActor's%20level) 4) Quest%20or%20enemy%20Level) ; is greater by 4?
            (LocalVariables|SetExp%20Gain%20Rate 0.2)
            (else
              (LocalVariables|SetExp%20Gain%20Rate 0.0))))))
    (else
      (LocalVariables|SetExp%20Gain%20Rate 1.0)))
  ;[1 1 1] Grant player the exp
  (bind _output_get (Variables|Actor'sStats|SetActor's%20experience (+ (Variables|Actor'sStats|GetActor's%20experience) (* (LocalVariables|GetExp%20Gain%20Rate) EXP%20To%20be%20gained))))
  ;[1 1 1] Check if Player should lv up
  (if (> _output_get 1e+03)
    ;[1 1 1] Level++
    (Variables|Actor'sStats|SetActor's%20level (+ (Variables|Actor'sStats|GetActor's%20level) 1))
    ;[1 1 1] add Overboard exp to Player's Exp
    (Variables|Actor'sStats|SetActor's%20experience (- _output_get 1e+03))))

(fn ReceiveWeaponDamage
  (params (PhysicalDamage :type Float%20%28double-precision%29) (MagicalDamage :type Float%20%28double-precision%29))
  (bind _returnvalue (* PhysicalDamage 0.1))
  (bind _returnvalue_2 (* MagicalDamage 0.1))
  (bind _armour (Variables|DefenceStats|GetArmour))
  (bind _magicresistance (Variables|DefenceStats|GetMagicResistance))
  (bind _returnvalue_3 (- PhysicalDamage _armour))
  (bind _returnvalue_4 (+ _returnvalue _returnvalue_2))
  (bind _returnvalue_5 (- _magicresistance MagicalDamage))
  (bind _returnvalue_6 (Math|Float|Min(Float) _returnvalue_5 0.0))
  (bind _returnvalue_7 (Math|Float|Min(Float) _returnvalue_3 0.0))
  (bind _returnvalue_8 (+ _returnvalue_7 _returnvalue_6))
  (if (> _returnvalue_8 _returnvalue_4)
    ;[1 1 1] Deals normal damage ammount
    (Variables|Actor'sbasicstats|SetCurrentHp (- (Variables|Actor'sbasicstats|GetCurrentHp) _returnvalue_8))
    (else
      ;[1 1 1] Deals minimal damage ammount
      (Variables|Actor'sbasicstats|SetCurrentHp (- (Variables|Actor'sbasicstats|GetCurrentHp) _returnvalue_4)))))

(fn TurnonRagDoll
  (bind _returnvalue (Components|GetOwner))
  (bind _skeletalmeshcomponent (Class|BPICharacterBase|GetSkeletalMeshComponent(Message) _returnvalue))
  (bind _charactermovementcomponent (Class|BPICharacterBase|GetCharacterMovementComponent(Message) _returnvalue))
  (Physics|SetSimulatePhysics _skeletalmeshcomponent true)
  (Pawn|Components|CharacterMovement|DisableMovement _charactermovementcomponent))

(fn TurnOffRagDoll
  (bind _returnvalue (Components|GetOwner))
  (bind _skeletalmeshcomponent (Class|BPICharacterBase|GetSkeletalMeshComponent(Message) _returnvalue))
  (bind _charactermovementcomponent (Class|BPICharacterBase|GetCharacterMovementComponent(Message) _returnvalue))
  (Physics|SetSimulatePhysics _skeletalmeshcomponent false)
  ;[1 0 0] Test This to Enable movement component
  (Pawn|Components|CharacterMovement|SetMovementMode _charactermovementcomponent "MOVE_Walking" 0))

(fn SetMaxHpMpSp
  (params (RestLevel :type Float%20%28double-precision%29))
  (bind _actor_s_level (Variables|Actor'sStats|GetActor's%20level))
  (bind _returnvalue (Math|Conversions|ToFloat(Byte) _actor_s_level))
  (bind _returnvalue_2 (* _returnvalue 5.0))
  (Variables|Actor'sbasicstats|SetMaxHp (* (Math|Float|Max(Float) (* _returnvalue_2 (Math|Float|Max(Float) (/ (Math|Conversions|ToFloat(Byte) (Variables|Actor'sBasicStats|GetPhysique)) 1e+01) 1.0)) 1e+01) RestLevel))
  (Variables|Actor'sbasicstats|SetMaxMp (* (Math|Float|Max(Float) (* _returnvalue_2 (Math|Float|Max(Float) (/ (Math|Conversions|ToFloat(Byte) (Variables|Actor'sBasicStats|GetWill)) 1e+01) 1.0)) 1e+01) RestLevel))
  (Variables|Actor'sbasicstats|SetMaxSp (* (Math|Float|Max(Float) (* _returnvalue_2 (Math|Float|Max(Float) (/ (Math|Conversions|ToFloat(Byte) (Variables|Actor'sBasicStats|GetEndurance)) 1e+01) 1.0)) 1e+01) RestLevel)))

(fn SetRegen
  (params (RestLevel :type Float%20%28double-precision%29))
  (bind _actor_s_level (Variables|Actor'sStats|GetActor's%20level))
  (bind _returnvalue (Math|Conversions|ToFloat(Byte) _actor_s_level))
  (bind _returnvalue_2 (* _returnvalue 0.5))
  ;[1 1 1] How much  of that  stat will be regenerated per every 5  secs
  (Variables|Actor'sBasicStats|SetHpRegen (* (* _returnvalue_2 (Math|Float|Max(Float) (/ (Math|Conversions|ToFloat(Byte) (Variables|Actor'sBasicStats|GetWoundClotting)) 2e+01) 1.0)) RestLevel))
  (Variables|Actor'sBasicStats|SetMpRegen (* (* _returnvalue_2 (Math|Float|Max(Float) (/ (Math|Conversions|ToFloat(Byte) (Variables|Actor'sBasicStats|GetMindPeace)) 1e+01) 1.0)) RestLevel))
  (Variables|Actor'sBasicStats|SetSpRegen (* (* _returnvalue_2 (Math|Float|Max(Float) (/ (Math|Conversions|ToFloat(Byte) 0) 1e+01) 1.0)) RestLevel)))

(fn SetDamage
  (params (RestLevel :type Float%20%28double-precision%29))
  ;[1 1 1] Multiplier damage of weapon by the perk efficency
  ; DMG = WeaponDamage*(Perk/10)
  (bind (_rmb _lmb) (Class|BPICharacterBase|GetEquippedWeapon(Message) (Components|GetOwner)))
  (switch Utilities|FlowControl|Switch|SwitchonE_WeaponType (.WeaponType (Utilities|Struct|BreakS_WeaponInfo _rmb))
    (:NewEnumerator0
      (LocalVariables|SetMultiplier (* (/ (Math|Conversions|ToFloat(Byte) (Variables|CombatPerks|Get1Handed)) 1e+01) RestLevel)))
    (:NewEnumerator1
      (LocalVariables|SetMultiplier (* (/ (Math|Conversions|ToFloat(Byte) (Variables|CombatPerks|Get2Handed)) 1e+01) RestLevel)))
    (:NewEnumerator3
      (LocalVariables|SetMultiplier (* (/ (Math|Conversions|ToFloat(Byte) (Variables|CombatPerks|GetSpears)) 1e+01) RestLevel)))
    (:NewEnumerator2
      (LocalVariables|SetMultiplier (* (/ (Math|Conversions|ToFloat(Byte) (Variables|CombatPerks|GetGauntlets)) 1e+01) RestLevel))))
  ;[1 1 1] If eventualy I will decide there will be more damage types
  ; -Create Enum instead of bool E_DamageType
  (if (.DamageType (Utilities|Struct|BreakS_WeaponInfo _rmb))
    (Variables|RMBOffenceStats|SetRMB_MagicalDamage (* (.Damage (Utilities|Struct|BreakS_WeaponInfo _rmb)) (LocalVariables|GetMultiplier)))
    (Variables|RMBOffenceStats|SetRMB_PhysicalDamage 0.0)
    (else
      (Variables|RMBOffenceStats|SetRMB_PhysicalDamage (* (.Damage (Utilities|Struct|BreakS_WeaponInfo _rmb)) (LocalVariables|GetMultiplier)))
      (Variables|RMBOffenceStats|SetRMB_MagicalDamage 0.0)))
  (switch Utilities|FlowControl|Switch|SwitchonE_WeaponType (.WeaponType (Utilities|Struct|BreakS_WeaponInfo _lmb))
    (:NewEnumerator0
      (LocalVariables|SetMultiplier (* (/ (Math|Conversions|ToFloat(Byte) (Variables|CombatPerks|Get1Handed)) 1e+01) RestLevel)))
    (:NewEnumerator1
      (LocalVariables|SetMultiplier (* (/ (Math|Conversions|ToFloat(Byte) (Variables|CombatPerks|Get2Handed)) 1e+01) RestLevel)))
    (:NewEnumerator3
      (LocalVariables|SetMultiplier (* (/ (Math|Conversions|ToFloat(Byte) (Variables|CombatPerks|GetSpears)) 1e+01) RestLevel)))
    (:NewEnumerator2
      (LocalVariables|SetMultiplier (* (/ (Math|Conversions|ToFloat(Byte) (Variables|CombatPerks|GetGauntlets)) 1e+01) RestLevel))))
  (if (.DamageType (Utilities|Struct|BreakS_WeaponInfo _lmb))
    (Variables|LMBOffenceStats|SetLMB_MagicalDamage (* (.Damage (Utilities|Struct|BreakS_WeaponInfo _lmb)) (LocalVariables|GetMultiplier)))
    (Variables|LMBOffenceStats|SetLMB_PhysicalDamage 0.0)
    (else
      (Variables|LMBOffenceStats|SetLMB_PhysicalDamage (* (.Damage (Utilities|Struct|BreakS_WeaponInfo _lmb)) (LocalVariables|GetMultiplier)))
      (Variables|LMBOffenceStats|SetLMB_MagicalDamage 0.0))))

(fn CalculateRestMultiplier
  ;[1 1 1] Most of the time it will be at 1.1
  ; But after long time it will fall to as low as 0.5
  (return (Math|Float|Max(Float) (/ (Class|KismetMathLibrary|BMin (Variables|Actor'sStats|GetrestLevel) 110) 1e+02) 0.5)))

(fn SetInitialHpMpSp
  (params (RestLevel :type Float%20%28double-precision%29))
  (bind _actor_s_level (Variables|Actor'sStats|GetActor's%20level))
  (bind _returnvalue (Math|Conversions|ToFloat(Byte) _actor_s_level))
  (bind _returnvalue_2 (* _returnvalue 5.0))
  (bind _output_get (Variables|Actor'sbasicstats|SetMaxHp (* (Math|Float|Max(Float) (* _returnvalue_2 (Math|Float|Max(Float) (/ (Math|Conversions|ToFloat(Byte) (Variables|Actor'sBasicStats|GetPhysique)) 1e+01) 1.0)) 1e+01) RestLevel)))
  (bind _output_get_2 (Variables|Actor'sbasicstats|SetMaxMp (* (Math|Float|Max(Float) (* _returnvalue_2 (Math|Float|Max(Float) (/ (Math|Conversions|ToFloat(Byte) (Variables|Actor'sBasicStats|GetWill)) 1e+01) 1.0)) 1e+01) RestLevel)))
  (bind _output_get_3 (Variables|Actor'sbasicstats|SetMaxSp (* (Math|Float|Max(Float) (* _returnvalue_2 (Math|Float|Max(Float) (/ (Math|Conversions|ToFloat(Byte) (Variables|Actor'sBasicStats|GetEndurance)) 1e+01) 1.0)) 1e+01) RestLevel)))
  ;[1 1 1] Sets current  hp  to match
  (Variables|Actor'sbasicstats|SetCurrentHp _output_get)
  (Variables|Actor'sbasicstats|SetCurrentMp _output_get_2)
  (Variables|Actor'sbasicstats|SetCurrentSp _output_get_3))

(fn Level
  (return (Variables|Actor'sStats|GetActor's%20level)))