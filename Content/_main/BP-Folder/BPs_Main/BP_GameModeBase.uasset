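; Game mode that runs the in-game clock and day/night cycle, tracking real and game seconds played.
; A Timeline event track advances game time by a multiplier each tick, and SetSunPosition converts it into Sun and Moon rotations, with the moon offset.
; Time-skip events add time and reposition both bodies; waiting and no-rest skips drain the by-ref RestLevel at different rates, while short skips leave it untouched.
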(event EventBeginPlay
  (Utilities|FlowControl|Sequence
    (:then_0
      ;[1 1 1] Game time elaps
      (Timeline|Timeline_0 PlayFromStart ; Currently ticks every second
        (:EventTrack%20-%20Tick
          (Variables|DayNightcycle|SetIRL_SecondsPassed (+ (Variables|DayNightcycle|GetIRL_SecondsPassed) 1))
          (bind _output_get (Variables|DayNightCycle|SetGameSecondsPassed (+ (Variables|DayNightCycle|GetGameSecondsPassed) (Variables|DayNightCycle|GetGameTimeMultiplier))))
          (Day-Nightcycle|SetSunPosition _output_get))))))

(event EventTick
  (params (DeltaSeconds :type Float%20%28single-precision%29)))

(event EventSkipTimeWaiting
  (params (Hours%20amount :type Integer) (RestLevel :type Byte :default 0))
  ;[1 1 1] Intended for time skips where player can semi rest.
  ; It drains restLevel slower than normal gameplay
  (Day-NightCycle|SkipGameTimeWaiting 0 0 Hours%20amount RestLevel))

(event EventSkipTimeShort
  (params (Seconds :type Integer) (Minutes :type Integer))
  ;[1 1 1] Intended for Short time amount skips. Minutes and seconds.
  ; It shouldnt affect players restLevel so for performance sake it's not calculated here
  (Day-NightCycle|SkipGameTimeShort Seconds Minutes))

(event EventSkipTimeNoRest
  (params (Seconds :type Integer) (Minutes :type Integer) (Hours :type Integer) (Rest :type Byte%20%28by%20ref%29 :default 0))
  ;[1 1 1] Intended for skiping time when player will not rest
  ; It drains restLevel as if player were playing normally all this time
  (Day-NightCycle|SkipGameTimeNoRest Seconds Minutes Hours Rest))

(fn ConstructionScript
  (bind _returnvalue (Actor|GetActorOfClass "/Game/_main/BP-Folder/BPs_Main/Lighting/BP_Sun.BP_Sun_C"))
  (Variables|DayNightCycle|SetSun _returnvalue)
  (bind _returnvalue_2 (Actor|GetActorOfClass "/Game/_main/BP-Folder/BPs_Main/Lighting/BP_Moon.BP_Moon_C"))
  (Variables|DayNightCycle|SetMoon _returnvalue_2))

(fn SetSunPosition
  (params (GameSeconds :type Integer))
  (bind _returnvalue (/ GameSeconds 60))
  (bind _returnvalue_2 (* _returnvalue 0.25))
  (bind _returnvalue_3 (Math|Float|%(Float) _returnvalue_2 3.6e+02))
  (Transformation|SetActorRotation (Variables|DayNightCycle|GetSun) (Math|Rotator|MakeRotator 0.0 (+ _returnvalue_3 6e+01) 0.0))
  ;[1 1 1] Moon Rotation
  (Transformation|SetActorRotation (Variables|DayNightCycle|GetMoon) (Math|Rotator|MakeRotator 0.0 (+ (+ _returnvalue_3 165.0) 6e+01) 0.0))
  (Development|PrintString (Utilities|String|BuildString(Integer) "" "Hour is:" (/ (Math|Float|Truncate _returnvalue_3) 15)))
  (return))

(fn IRLTimeSpent
  (bind _irl_secondspassed (Variables|DayNightcycle|GetIRL_SecondsPassed))
  (bind _returnvalue (/ _irl_secondspassed 60))
  (Development|PrintString "Time spent  in game:")
  (Development|PrintString (Utilities|String|BuildString(Integer) "" "Hours: " (/ _returnvalue 60)))
  (Development|PrintString (Utilities|String|BuildString(Integer) "" "Minutes: " (Math|Integer|%(Integer) _returnvalue 60)))
  (Development|PrintString (Utilities|String|BuildString(Integer) "" "Seconds: " (Math|Integer|%(Integer) _irl_secondspassed 60))))

(fn SkipGameTimeWaiting
  (params (secondsAmmount :type Integer) (MinutesAmmount :type Integer) (HoursAmmount :type Integer) (RestLevel :type Byte%20%28by%20ref%29))
  (bind _returnvalue (* HoursAmmount 60))
  (bind _returnvalue_2 (+ MinutesAmmount _returnvalue))
  (bind _returnvalue_3 (* _returnvalue_2 60))
  (bind _returnvalue_4 (+ secondsAmmount _returnvalue_3))
  (bind _output_get (Variables|DayNightCycle|SetGameSecondsPassed (+ (Variables|DayNightCycle|GetGameSecondsPassed) _returnvalue_4)))
  (Day-Nightcycle|SetSunPosition _output_get)
  (|SetBy-RefVar RestLevel (- RestLevel (Math|Conversions|ToByte(Integer) (* (/ _returnvalue_4 120) 3))))
  (return))

(fn SkipGameTimeShort
  (params (secondsAmmount :type Integer) (MinutesAmmount :type Integer) (HoursAmmount :type Integer))
  (bind _output_get (Variables|DayNightCycle|SetGameSecondsPassed (+ (Variables|DayNightCycle|GetGameSecondsPassed) (+ secondsAmmount (* (+ MinutesAmmount (* HoursAmmount 60)) 60)))))
  (Day-Nightcycle|SetSunPosition _output_get)
  (return))

(fn SkipGameTimeNoRest
  (params (secondsAmmount :type Integer) (MinutesAmmount :type Integer) (HoursAmmount :type Integer) (RestLevel :type Byte%20%28by%20ref%29))
  (bind _returnvalue (* HoursAmmount 60))
  (bind _returnvalue_2 (+ MinutesAmmount _returnvalue))
  (bind _returnvalue_3 (* _returnvalue_2 60))
  (bind _returnvalue_4 (+ secondsAmmount _returnvalue_3))
  (bind _output_get (Variables|DayNightCycle|SetGameSecondsPassed (+ (Variables|DayNightCycle|GetGameSecondsPassed) _returnvalue_4)))
  (Day-Nightcycle|SetSunPosition _output_get)
  (|SetBy-RefVar RestLevel (- RestLevel (Math|Conversions|ToByte(Integer) (* (/ _returnvalue_4 120) 5))))
  (return))