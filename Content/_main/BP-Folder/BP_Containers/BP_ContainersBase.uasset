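; Base Blueprint for container actors, holding an InventoryComponent with category inventories for weapons, clothing, food, alchemy, crafting and junk.
; Getter functions expose the component and its category inventories.
; BeginPlay stores the StaticMesh in a PrimitiveComponent variable.
; DestroyAnActor clears the actor's tags and hides the mesh, then destroys the actor after a short delay.
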(event EventBeginPlay
  (Variables|Default|SetprimitiveComponent (Variables|Default|GetStaticMesh)))

(event Collision|EventActorBeginOverlap
  (params (OtherActor :type Actor%20Object%20Reference))
  (|CallParentFunction OtherActor) ; This node is disabled and will not be called.\nDrag off pins to build functionality.
)

(event EventTick
  (params (DeltaSeconds :type Float%20%28single-precision%29))
  (|CallParentFunction DeltaSeconds) ; This node is disabled and will not be called.\nDrag off pins to build functionality.
)

(event EventDestroyAnActor
  ;[1 1 1] This is just to avoid an error - I can delete this nodes
  (Utilities|Array|Clear (Variables|Default|GetTags))
  (Rendering|SetVisibility (Variables|Default|GetStaticMesh) false false)
  (Utilities|FlowControl|Delay 0.8)
  (Actor|DestroyActor self))

(fn ConstructionScript
  (|CallParentFunction))

(fn GetContainerInventory
  (bind _inventorycomponent (Variables|Default|GetInventoryComponent))
  (return (Variables|/Game/_main/BP-Folder/BPs_Base/InventoryComponent.InventoryComponent_C|GetInventoryWeapons _inventorycomponent) (Variables|/Game/_main/BP-Folder/BPs_Base/InventoryComponent.InventoryComponent_C|GetInventory_Clothing _inventorycomponent) (Variables|/Game/_main/BP-Folder/BPs_Base/InventoryComponent.InventoryComponent_C|GetInventoryFood _inventorycomponent) (Variables|/Game/_main/BP-Folder/BPs_Base/InventoryComponent.InventoryComponent_C|GetInventoryAlchemy _inventorycomponent) (Variables|/Game/_main/BP-Folder/BPs_Base/InventoryComponent.InventoryComponent_C|GetInventoryCrafting _inventorycomponent) (Variables|/Game/_main/BP-Folder/BPs_Base/InventoryComponent.InventoryComponent_C|GetInventoryJunk _inventorycomponent)))

(fn GetInventoryComponent
  (return (Variables|Default|GetInventoryComponent)))