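; BP_LootContainer is a loot container actor that merges with nearby containers of the same class.
; A sphere overlap triggers a randomly delayed scan of overlapping containers.
; Per-category Handle functions sum the other container's six inventory maps into its own, then the other is destroyed and the scan repeats.
; An IsAdded flag marks containers being absorbed; a flagged container waits, clears the flags and rescans instead of merging.
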(event OnComponentBeginOverlap(Sphere)
  (params (OverlappedComponent :type Primitive%20Component%20Object%20Reference) (OtherActor :type Actor%20Object%20Reference) (OtherComp :type Primitive%20Component%20Object%20Reference) (OtherBodyIndex :type Integer) (bFromSweep :type Boolean) (SweepResult :type Hit%20Result%20Structure%20%28by%20ref%29))
  (Utilities|FlowControl|Delay (Math|Random|RandomFloatinRange 0.0 5.0))
  (for _array_element (Collision|GetOverlappingActors (Variables|Components|GetSphere) "BP_LootContainer_C" :!class /Script/Engine.PrimitiveComponent)
    ;[1 0.01317 0] TODO - Merge close DropContainers Into one
    (bind _asbp_loot_container (Utilities|Casting|CastToBP_LootContainer _array_element)
      (:then
        (Variables|BP_LootContainer_C|SetisAdded _asbp_loot_container true)
        (if (Variables|Default|GetisAdded)
          (Utilities|FlowControl|Delay (Math|Random|RandomFloatinRange 5.1 1e+01))
          (Variables|BP_LootContainer_C|SetisAdded _asbp_loot_container false)
          (Variables|Default|SetisAdded false)
          (CallFunction|CheckOverlappedAgain)
          (else
            (bind _reference (Default|GetDropContainerReference _asbp_loot_container))
            ;[1 1 1] sprawdz czy cos w ogole jest w mapie
            (if (== (Utilities|Map|Length (Variables|/Game/_main/BP-Folder/BPs_Main/InventoryComponent.InventoryComponent_C|GetInventoryWeapons (Variables|/Game/_main/BP-Folder/BP_Containers/BP_ContainersBase.BP_ContainersBase_C|GetInventoryComponent _reference))) 0)
              _
              (else
                ;[1 1 1] Znajdz klucz i value --> dodaj je do swojej mapy
                (CallFunction|HandleWeapons (Variables|/Game/_main/BP-Folder/BPs_Main/InventoryComponent.InventoryComponent_C|GetInventoryWeapons (Variables|/Game/_main/BP-Folder/BP_Containers/BP_ContainersBase.BP_ContainersBase_C|GetInventoryComponent _reference)))))
            (if (== (Utilities|Map|Length (Variables|/Game/_main/BP-Folder/BPs_Main/InventoryComponent.InventoryComponent_C|GetInventory_Clothing (Variables|/Game/_main/BP-Folder/BP_Containers/BP_ContainersBase.BP_ContainersBase_C|GetInventoryComponent _reference))) 0)
              _
              (else
                (CallFunction|HandleClothing (Variables|/Game/_main/BP-Folder/BPs_Main/InventoryComponent.InventoryComponent_C|GetInventory_Clothing (Variables|/Game/_main/BP-Folder/BP_Containers/BP_ContainersBase.BP_ContainersBase_C|GetInventoryComponent _reference)))))
            (if (== (Utilities|Map|Length (Variables|/Game/_main/BP-Folder/BPs_Main/InventoryComponent.InventoryComponent_C|GetInventoryFood (Variables|/Game/_main/BP-Folder/BP_Containers/BP_ContainersBase.BP_ContainersBase_C|GetInventoryComponent _reference))) 0)
              _
              (else
                (CallFunction|HandleFood (Variables|/Game/_main/BP-Folder/BPs_Main/InventoryComponent.InventoryComponent_C|GetInventoryFood (Variables|/Game/_main/BP-Folder/BP_Containers/BP_ContainersBase.BP_ContainersBase_C|GetInventoryComponent _reference)))))
            (if (== (Utilities|Map|Length (Variables|/Game/_main/BP-Folder/BPs_Main/InventoryComponent.InventoryComponent_C|GetInventoryAlchemy (Variables|/Game/_main/BP-Folder/BP_Containers/BP_ContainersBase.BP_ContainersBase_C|GetInventoryComponent _reference))) 0)
              _
              (else
                (CallFunction|HandleAlchemy (Variables|/Game/_main/BP-Folder/BPs_Main/InventoryComponent.InventoryComponent_C|GetInventoryAlchemy (Variables|/Game/_main/BP-Folder/BP_Containers/BP_ContainersBase.BP_ContainersBase_C|GetInventoryComponent _reference)))))
            (if (== (Utilities|Map|Length (Variables|/Game/_main/BP-Folder/BPs_Main/InventoryComponent.InventoryComponent_C|GetInventoryCrafting (Variables|/Game/_main/BP-Folder/BP_Containers/BP_ContainersBase.BP_ContainersBase_C|GetInventoryComponent _reference))) 0)
              _
              (else
                (CallFunction|HandleCrafting (Variables|/Game/_main/BP-Folder/BPs_Main/InventoryComponent.InventoryComponent_C|GetInventoryCrafting (Variables|/Game/_main/BP-Folder/BP_Containers/BP_ContainersBase.BP_ContainersBase_C|GetInventoryComponent _reference)))))
            (if (== (Utilities|Map|Length (Variables|/Game/_main/BP-Folder/BPs_Main/InventoryComponent.InventoryComponent_C|GetInventoryJunk (Variables|/Game/_main/BP-Folder/BP_Containers/BP_ContainersBase.BP_ContainersBase_C|GetInventoryComponent _reference))) 0)
              _
              (else
                (CallFunction|HandleJunk (Variables|/Game/_main/BP-Folder/BPs_Main/InventoryComponent.InventoryComponent_C|GetInventoryJunk (Variables|/Game/_main/BP-Folder/BP_Containers/BP_ContainersBase.BP_ContainersBase_C|GetInventoryComponent _reference)))))
            ;[1 1 1] zniszcz dodany obiekt
            (Default|DestroyAnActor _asbp_loot_container)
            ;[1 1 1] Sprawdz inne mapy
            (CallFunction|CheckOverlappedAgain))))
      (:CastFailed
        (Development|PrintString "Cast Failed in BP_DropDontainer")))))

(event Custom|check%20overlapped%20again
  (Utilities|FlowControl|Delay (Math|Random|RandomFloatinRange 0.0 5.0))
  (for _array_element (Collision|GetOverlappingActors (Variables|Components|GetSphere) "BP_LootContainer_C" :!class /Script/Engine.PrimitiveComponent)
    ;[1 0.01317 0] TODO - Merge close DropContainers Into one
    (bind _asbp_loot_container (Utilities|Casting|CastToBP_LootContainer _array_element)
      (:then
        (Variables|BP_LootContainer_C|SetisAdded _asbp_loot_container true)
        (if (Variables|Default|GetisAdded)
          (Utilities|FlowControl|Delay (Math|Random|RandomFloatinRange 5.1 1e+01))
          (Variables|BP_LootContainer_C|SetisAdded _asbp_loot_container false)
          (Variables|Default|SetisAdded false)
          (CallFunction|CheckOverlappedAgain)
          (else
            (bind _reference (Default|GetDropContainerReference _asbp_loot_container))
            ;[1 1 1] sprawdz czy cos w ogole jest w mapie
            (if (== (Utilities|Map|Length (Variables|/Game/_main/BP-Folder/BPs_Main/InventoryComponent.InventoryComponent_C|GetInventoryWeapons (Variables|/Game/_main/BP-Folder/BP_Containers/BP_ContainersBase.BP_ContainersBase_C|GetInventoryComponent _reference))) 0)
              _
              (else
                ;[1 1 1] Znajdz klucz i value --> dodaj je do swojej mapy
                (CallFunction|HandleWeapons (Variables|/Game/_main/BP-Folder/BPs_Main/InventoryComponent.InventoryComponent_C|GetInventoryWeapons (Variables|/Game/_main/BP-Folder/BP_Containers/BP_ContainersBase.BP_ContainersBase_C|GetInventoryComponent _reference)))))
            (if (== (Utilities|Map|Length (Variables|/Game/_main/BP-Folder/BPs_Main/InventoryComponent.InventoryComponent_C|GetInventory_Clothing (Variables|/Game/_main/BP-Folder/BP_Containers/BP_ContainersBase.BP_ContainersBase_C|GetInventoryComponent _reference))) 0)
              _
              (else
                (CallFunction|HandleClothing (Variables|/Game/_main/BP-Folder/BPs_Main/InventoryComponent.InventoryComponent_C|GetInventory_Clothing (Variables|/Game/_main/BP-Folder/BP_Containers/BP_ContainersBase.BP_ContainersBase_C|GetInventoryComponent _reference)))))
            (if (== (Utilities|Map|Length (Variables|/Game/_main/BP-Folder/BPs_Main/InventoryComponent.InventoryComponent_C|GetInventoryFood (Variables|/Game/_main/BP-Folder/BP_Containers/BP_ContainersBase.BP_ContainersBase_C|GetInventoryComponent _reference))) 0)
              _
              (else
                (CallFunction|HandleFood (Variables|/Game/_main/BP-Folder/BPs_Main/InventoryComponent.InventoryComponent_C|GetInventoryFood (Variables|/Game/_main/BP-Folder/BP_Containers/BP_ContainersBase.BP_ContainersBase_C|GetInventoryComponent _reference)))))
            (if (== (Utilities|Map|Length (Variables|/Game/_main/BP-Folder/BPs_Main/InventoryComponent.InventoryComponent_C|GetInventoryAlchemy (Variables|/Game/_main/BP-Folder/BP_Containers/BP_ContainersBase.BP_ContainersBase_C|GetInventoryComponent _reference))) 0)
              _
              (else
                (CallFunction|HandleAlchemy (Variables|/Game/_main/BP-Folder/BPs_Main/InventoryComponent.InventoryComponent_C|GetInventoryAlchemy (Variables|/Game/_main/BP-Folder/BP_Containers/BP_ContainersBase.BP_ContainersBase_C|GetInventoryComponent _reference)))))
            (if (== (Utilities|Map|Length (Variables|/Game/_main/BP-Folder/BPs_Main/InventoryComponent.InventoryComponent_C|GetInventoryCrafting (Variables|/Game/_main/BP-Folder/BP_Containers/BP_ContainersBase.BP_ContainersBase_C|GetInventoryComponent _reference))) 0)
              _
              (else
                (CallFunction|HandleCrafting (Variables|/Game/_main/BP-Folder/BPs_Main/InventoryComponent.InventoryComponent_C|GetInventoryCrafting (Variables|/Game/_main/BP-Folder/BP_Containers/BP_ContainersBase.BP_ContainersBase_C|GetInventoryComponent _reference)))))
            (if (== (Utilities|Map|Length (Variables|/Game/_main/BP-Folder/BPs_Main/InventoryComponent.InventoryComponent_C|GetInventoryJunk (Variables|/Game/_main/BP-Folder/BP_Containers/BP_ContainersBase.BP_ContainersBase_C|GetInventoryComponent _reference))) 0)
              _
              (else
                (CallFunction|HandleJunk (Variables|/Game/_main/BP-Folder/BPs_Main/InventoryComponent.InventoryComponent_C|GetInventoryJunk (Variables|/Game/_main/BP-Folder/BP_Containers/BP_ContainersBase.BP_ContainersBase_C|GetInventoryComponent _reference)))))
            ;[1 1 1] zniszcz dodany obiekt
            (Default|DestroyAnActor _asbp_loot_container)
            ;[1 1 1] Sprawdz inne mapy
            (CallFunction|CheckOverlappedAgain))))
      (:CastFailed
        (Development|PrintString "Cast Failed in BP_DropDontainer")))))

(event EventBeginPlay
  (|CallParentFunction))

(event Collision|EventActorBeginOverlap
  (params (OtherActor :type Actor%20Object%20Reference))
  (|CallParentFunction OtherActor) ; This node is disabled and will not be called.\nDrag off pins to build functionality.
)

(event EventTick
  (params (DeltaSeconds :type Float%20%28single-precision%29))
  (|CallParentFunction DeltaSeconds) ; This node is disabled and will not be called.\nDrag off pins to build functionality.
)

(fn ConstructionScript
  (|CallParentFunction))

(fn HandleWeapons
  (params (WeaponInventory :type Map%20of%20S%20Weapon%20Info%20Structures%20to%20Integers))
  (bind _inventorycomponent (Variables|Default|GetInventoryComponent))
  (bind _inventoryweapons (Variables|/Game/_main/BP-Folder/BPs_Main/InventoryComponent.InventoryComponent_C|GetInventoryWeapons _inventorycomponent))
  (bind _keys (Utilities|Map|Keys WeaponInventory))
  (bind _values (Utilities|Map|Values WeaponInventory))
  (for (_array_element _array_index) _keys
    (if (.ReturnValue (Utilities|Map|Find _inventoryweapons _array_element))
      (Utilities|Map|Add _inventoryweapons _array_element (+ (.Value (Utilities|Map|Find _inventoryweapons _array_element)) (Utilities|Array|Get(acopy) _values _array_index)))
      (else
        (Utilities|Map|Add _inventoryweapons _array_element (Utilities|Array|Get(acopy) _values _array_index))))
    (Utilities|Map|Remove WeaponInventory _array_element))
  (return))

(fn HandleClothing
  (params (ClothingInventory :type Map%20of%20S%20Clothing%20Info%20Structures%20to%20Integers))
  (bind _inventorycomponent (Variables|Default|GetInventoryComponent))
  (bind _inventory_clothing (Variables|/Game/_main/BP-Folder/BPs_Main/InventoryComponent.InventoryComponent_C|GetInventory_Clothing _inventorycomponent))
  (bind _keys (Utilities|Map|Keys ClothingInventory))
  (bind _values (Utilities|Map|Values ClothingInventory))
  (for (_array_element _array_index) _keys
    (if (.ReturnValue (Utilities|Map|Find _inventory_clothing _array_element))
      (Utilities|Map|Add _inventory_clothing _array_element (+ (.Value (Utilities|Map|Find _inventory_clothing _array_element)) (Utilities|Array|Get(acopy) _values _array_index)))
      (else
        (Utilities|Map|Add _inventory_clothing _array_element (Utilities|Array|Get(acopy) _values _array_index))))
    (Utilities|Map|Remove ClothingInventory _array_element))
  (return))

(fn HandleJunk
  (params (JunkInventory :type Map%20of%20S%20Junk%20Info%20Structures%20to%20Integers))
  (bind _inventorycomponent (Variables|Default|GetInventoryComponent))
  (bind _inventoryjunk (Variables|/Game/_main/BP-Folder/BPs_Main/InventoryComponent.InventoryComponent_C|GetInventoryJunk _inventorycomponent))
  (bind _keys (Utilities|Map|Keys JunkInventory))
  (bind _values (Utilities|Map|Values JunkInventory))
  (for (_array_element _array_index) _keys
    (if (.ReturnValue (Utilities|Map|Find _inventoryjunk _array_element))
      (Utilities|Map|Add _inventoryjunk _array_element (+ (.Value (Utilities|Map|Find _inventoryjunk _array_element)) (Utilities|Array|Get(acopy) _values _array_index)))
      (else
        (Utilities|Map|Add _inventoryjunk _array_element (Utilities|Array|Get(acopy) _values _array_index))))
    (Utilities|Map|Remove JunkInventory _array_element))
  (return))

(fn HandleFood
  (params (FoodInventory :type Map%20of%20S%20Food%20Info%20Structures%20to%20Integers))
  (bind _inventorycomponent (Variables|Default|GetInventoryComponent))
  (bind _inventoryfood (Variables|/Game/_main/BP-Folder/BPs_Main/InventoryComponent.InventoryComponent_C|GetInventoryFood _inventorycomponent))
  (bind _keys (Utilities|Map|Keys FoodInventory))
  (bind _values (Utilities|Map|Values FoodInventory))
  (for (_array_element _array_index) _keys
    (if (.ReturnValue (Utilities|Map|Find _inventoryfood _array_element))
      (Utilities|Map|Add _inventoryfood _array_element (+ (.Value (Utilities|Map|Find _inventoryfood _array_element)) (Utilities|Array|Get(acopy) _values _array_index)))
      (else
        (Utilities|Map|Add _inventoryfood _array_element (Utilities|Array|Get(acopy) _values _array_index))))
    (Utilities|Map|Remove FoodInventory _array_element))
  (return))

(fn HandleAlchemy
  (params (AlchemyInventory :type Map%20of%20S%20Alchemy%20Info%20Structures%20to%20Integers))
  (bind _inventorycomponent (Variables|Default|GetInventoryComponent))
  (bind _inventoryalchemy (Variables|/Game/_main/BP-Folder/BPs_Main/InventoryComponent.InventoryComponent_C|GetInventoryAlchemy _inventorycomponent))
  (bind _keys (Utilities|Map|Keys AlchemyInventory))
  (bind _values (Utilities|Map|Values AlchemyInventory))
  (for (_array_element _array_index) _keys
    (if (.ReturnValue (Utilities|Map|Find _inventoryalchemy _array_element))
      (Utilities|Map|Add _inventoryalchemy _array_element (+ (.Value (Utilities|Map|Find _inventoryalchemy _array_element)) (Utilities|Array|Get(acopy) _values _array_index)))
      (else
        (Utilities|Map|Add _inventoryalchemy _array_element (Utilities|Array|Get(acopy) _values _array_index))))
    (Utilities|Map|Remove AlchemyInventory _array_element))
  (return))

(fn HandleCrafting
  (params (CraftingInventory :type Map%20of%20S%20Crafting%20Info%20Structures%20to%20Integers))
  (bind _inventorycomponent (Variables|Default|GetInventoryComponent))
  (bind _inventorycrafting (Variables|/Game/_main/BP-Folder/BPs_Main/InventoryComponent.InventoryComponent_C|GetInventoryCrafting _inventorycomponent))
  (bind _keys (Utilities|Map|Keys CraftingInventory))
  (bind _values (Utilities|Map|Values CraftingInventory))
  (for (_array_element _array_index) _keys
    (if (.ReturnValue (Utilities|Map|Find _inventorycrafting _array_element))
      (Utilities|Map|Add _inventorycrafting _array_element (+ (.Value (Utilities|Map|Find _inventorycrafting _array_element)) (Utilities|Array|Get(acopy) _values _array_index)))
      (else
        (Utilities|Map|Add _inventorycrafting _array_element (Utilities|Array|Get(acopy) _values _array_index))))
    (Utilities|Map|Remove CraftingInventory _array_element))
  (return))

(fn GetDropContainerReference
  (return self))