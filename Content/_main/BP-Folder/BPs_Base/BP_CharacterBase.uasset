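; Base character Blueprint that handles HP, MP and SP regeneration, overhead-style chat text and common getters.
; A timeline started on BeginPlay or StartRegen periodically adds regen values from BPCBasicAttributes while alive, stopping when all three are full.
; ShowChatText fills a widget and returns a display time scaled by text length.
; GetEquippedWeapon and Level are stubs, and the slow resting timeline is unconnected.
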(event EventBeginPlay
  (bind _bpc_basicattributes (Variables|Default|GetBPC_BasicAttributes))
  (Utilities|FlowControl|Sequence
    (:then_0
      ;[1 0.5925 0.02034] Regenerate hp
      ;;[1 0 0.053] TODO Optimize ->Try to make Timeline off when all bars are full (full Hp&Mp&Sp)
      (Timeline|Timeline_0 PlayFromStart ; Currently ticks every 5 secs
        (:EventTrack%20-%20Tick
          ;;[1 1 1] When player is Dead do not regenerate
          (if (not (Variables|/Game/_main/BP-Folder/BPs_Base/BPC_BasicAttributes.BPC_BasicAttributes_C|GetIsDead _bpc_basicattributes))
            ;;[1 1 1] Regenerate Hp
            (Variables|/Game/_main/BP-Folder/BPs_Base/BPC_BasicAttributes.BPC_BasicAttributes_C|SetCurrentHp _bpc_basicattributes (Math|Float|Clamp(Float) (+ (Variables|/Game/_main/BP-Folder/BPs_Base/BPC_BasicAttributes.BPC_BasicAttributes_C|GetCurrentHp _bpc_basicattributes) (Variables|/Game/_main/BP-Folder/BPs_Base/BPC_BasicAttributes.BPC_BasicAttributes_C|GetHpRegen _bpc_basicattributes)) 0.0 (Variables|/Game/_main/BP-Folder/BPs_Base/BPC_BasicAttributes.BPC_BasicAttributes_C|GetMaxHp _bpc_basicattributes)))
            ;;[1 1 1] Regenerate Mp
            (Variables|/Game/_main/BP-Folder/BPs_Base/BPC_BasicAttributes.BPC_BasicAttributes_C|SetCurrentMp _bpc_basicattributes (Math|Float|Clamp(Float) (+ (Variables|/Game/_main/BP-Folder/BPs_Base/BPC_BasicAttributes.BPC_BasicAttributes_C|GetCurrentMp _bpc_basicattributes) (Variables|/Game/_main/BP-Folder/BPs_Base/BPC_BasicAttributes.BPC_BasicAttributes_C|GetMpRegen _bpc_basicattributes)) 0.0 (Variables|/Game/_main/BP-Folder/BPs_Base/BPC_BasicAttributes.BPC_BasicAttributes_C|GetMaxMp _bpc_basicattributes)))
            ;;[1 1 1] Regenerate Sp
            (Variables|/Game/_main/BP-Folder/BPs_Base/BPC_BasicAttributes.BPC_BasicAttributes_C|SetCurrentSp _bpc_basicattributes (Math|Float|Clamp(Float) (+ (Variables|/Game/_main/BP-Folder/BPs_Base/BPC_BasicAttributes.BPC_BasicAttributes_C|GetCurrentSp _bpc_basicattributes) (Variables|/Game/_main/BP-Folder/BPs_Base/BPC_BasicAttributes.BPC_BasicAttributes_C|GetSpRegen _bpc_basicattributes)) 0.0 (Variables|/Game/_main/BP-Folder/BPs_Base/BPC_BasicAttributes.BPC_BasicAttributes_C|GetMaxSp _bpc_basicattributes)))
            (Development|PrintString (Utilities|String|BuildString(Integer) (Utilities|GetObjectName self) " Hp: " (Math|Float|Truncate (Variables|/Game/_main/BP-Folder/BPs_Base/BPC_BasicAttributes.BPC_BasicAttributes_C|GetCurrentHp _bpc_basicattributes))))
            ;;[1 1 1] Stop regeneration(timeline) if all bars are  full
            ;; Untill I get damaged or use SP/MP
            (if (== (Variables|/Game/_main/BP-Folder/BPs_Base/BPC_BasicAttributes.BPC_BasicAttributes_C|GetMaxSp _bpc_basicattributes) (Variables|/Game/_main/BP-Folder/BPs_Base/BPC_BasicAttributes.BPC_BasicAttributes_C|GetCurrentSp _bpc_basicattributes))
              (if (== (Variables|/Game/_main/BP-Folder/BPs_Base/BPC_BasicAttributes.BPC_BasicAttributes_C|GetMaxHp _bpc_basicattributes) (Variables|/Game/_main/BP-Folder/BPs_Base/BPC_BasicAttributes.BPC_BasicAttributes_C|GetCurrentHp _bpc_basicattributes))
                (if (== (Variables|/Game/_main/BP-Folder/BPs_Base/BPC_BasicAttributes.BPC_BasicAttributes_C|GetMaxMp _bpc_basicattributes) (Variables|/Game/_main/BP-Folder/BPs_Base/BPC_BasicAttributes.BPC_BasicAttributes_C|GetCurrentMp _bpc_basicattributes))
                  (Timeline|Timeline_0 Stop))))))))))

(event Collision|EventActorBeginOverlap
  (params (OtherActor :type Actor%20Object%20Reference)))

(event EventTick
  (params (DeltaSeconds :type Float%20%28single-precision%29)))

(event EventStartRegen
  (bind _bpc_basicattributes (Variables|Default|GetBPC_BasicAttributes))
  ;[1 0.5925 0.02034] Regenerate hp
  ;;[1 1 1] Probably should Call this event whenever  Player
  ;; -Get Damaged
  ;; -Uses Mp/Hp/Sp
  ;; -levels up
  ;; -levels up a stat  related perk
  ;;[1 0 0.053] TODO Optimize ->Try to make Timeline off when all bars are full (full Hp&Mp&Sp)
  (Timeline|Timeline_0 PlayFromStart ; Currently ticks every 5 secs
    (:EventTrack%20-%20Tick
      ;;[1 1 1] When player is Dead do not regenerate
      (if (not (Variables|/Game/_main/BP-Folder/BPs_Base/BPC_BasicAttributes.BPC_BasicAttributes_C|GetIsDead _bpc_basicattributes))
        ;;[1 1 1] Regenerate Hp
        (Variables|/Game/_main/BP-Folder/BPs_Base/BPC_BasicAttributes.BPC_BasicAttributes_C|SetCurrentHp _bpc_basicattributes (Math|Float|Clamp(Float) (+ (Variables|/Game/_main/BP-Folder/BPs_Base/BPC_BasicAttributes.BPC_BasicAttributes_C|GetCurrentHp _bpc_basicattributes) (Variables|/Game/_main/BP-Folder/BPs_Base/BPC_BasicAttributes.BPC_BasicAttributes_C|GetHpRegen _bpc_basicattributes)) 0.0 (Variables|/Game/_main/BP-Folder/BPs_Base/BPC_BasicAttributes.BPC_BasicAttributes_C|GetMaxHp _bpc_basicattributes)))
        ;;[1 1 1] Regenerate Mp
        (Variables|/Game/_main/BP-Folder/BPs_Base/BPC_BasicAttributes.BPC_BasicAttributes_C|SetCurrentMp _bpc_basicattributes (Math|Float|Clamp(Float) (+ (Variables|/Game/_main/BP-Folder/BPs_Base/BPC_BasicAttributes.BPC_BasicAttributes_C|GetCurrentMp _bpc_basicattributes) (Variables|/Game/_main/BP-Folder/BPs_Base/BPC_BasicAttributes.BPC_BasicAttributes_C|GetMpRegen _bpc_basicattributes)) 0.0 (Variables|/Game/_main/BP-Folder/BPs_Base/BPC_BasicAttributes.BPC_BasicAttributes_C|GetMaxMp _bpc_basicattributes)))
        ;;[1 1 1] Regenerate Sp
        (Variables|/Game/_main/BP-Folder/BPs_Base/BPC_BasicAttributes.BPC_BasicAttributes_C|SetCurrentSp _bpc_basicattributes (Math|Float|Clamp(Float) (+ (Variables|/Game/_main/BP-Folder/BPs_Base/BPC_BasicAttributes.BPC_BasicAttributes_C|GetCurrentSp _bpc_basicattributes) (Variables|/Game/_main/BP-Folder/BPs_Base/BPC_BasicAttributes.BPC_BasicAttributes_C|GetSpRegen _bpc_basicattributes)) 0.0 (Variables|/Game/_main/BP-Folder/BPs_Base/BPC_BasicAttributes.BPC_BasicAttributes_C|GetMaxSp _bpc_basicattributes)))
        (Development|PrintString (Utilities|String|BuildString(Integer) (Utilities|GetObjectName self) " Hp: " (Math|Float|Truncate (Variables|/Game/_main/BP-Folder/BPs_Base/BPC_BasicAttributes.BPC_BasicAttributes_C|GetCurrentHp _bpc_basicattributes))))
        ;;[1 1 1] Stop regeneration(timeline) if all bars are  full
        ;; Untill I get damaged or use SP/MP
        (if (== (Variables|/Game/_main/BP-Folder/BPs_Base/BPC_BasicAttributes.BPC_BasicAttributes_C|GetMaxSp _bpc_basicattributes) (Variables|/Game/_main/BP-Folder/BPs_Base/BPC_BasicAttributes.BPC_BasicAttributes_C|GetCurrentSp _bpc_basicattributes))
          (if (== (Variables|/Game/_main/BP-Folder/BPs_Base/BPC_BasicAttributes.BPC_BasicAttributes_C|GetMaxHp _bpc_basicattributes) (Variables|/Game/_main/BP-Folder/BPs_Base/BPC_BasicAttributes.BPC_BasicAttributes_C|GetCurrentHp _bpc_basicattributes))
            (if (== (Variables|/Game/_main/BP-Folder/BPs_Base/BPC_BasicAttributes.BPC_BasicAttributes_C|GetMaxMp _bpc_basicattributes) (Variables|/Game/_main/BP-Folder/BPs_Base/BPC_BasicAttributes.BPC_BasicAttributes_C|GetCurrentMp _bpc_basicattributes))
              (Timeline|Timeline_0 Stop))))))))

(fn ConstructionScript)

(fn ShowChatText
  (params (text :type Text) (NewParam :type E_ChatColour%20Enum :default "NewEnumerator0"))
  (bind _widget (Variables|Default|GetWidget))
  (Rendering|SetVisibility _widget true false)
  (Class|BPIChat|SetChatText(Message) (UserInterface|GetUserWidgetObject _widget) text NewParam)
  (return (+ (* (Math|Conversions|ToFloat(Integer) (Utilities|String|Len (Utilities|String|ToString(Text) text))) 0.2) 1.2)))

(fn HideChatText
  (bind _widget (Variables|Default|GetWidget))
  (Rendering|SetVisibility _widget false false)
  (Class|BPIChat|SetChatText(Message) (UserInterface|GetUserWidgetObject _widget) "" "NewEnumerator0")
  (return))

(fn GetAttributeComponent
  (return (Variables|Default|GetBPC_BasicAttributes)))

(fn GetCharacterMovementComponent
  (return (Variables|Character|GetCharacterMovement)))

(fn GetCollisionCyllinder
  (return (Variables|Collision|GetCapsuleComponent)))

(fn GetEquippedWeapon
  (return "" ""))

(fn GetLocation
  (return (Transformation|GetActorLocation)))

(fn GetSkeletalMeshComponent
  (return (Variables|Character|GetMesh)))

(fn Level
  (return 0))