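; Actor component that holds a character's RPG combat attributes: HP/MP/SP, regen rates, damage, experience and level.
; RecalculateStats runs on BeginPlay, deriving maximums and regen from level and attributes and refilling current values; SetDamage is an unfinished weapon-type switch.
; GetHit applies armour-adjusted damage with a 10% floor, then ragdolls the owner at zero HP via interface messages.
; GainExp scales rewards down for lower-level sources and levels up every 1000 XP.
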(event Custom|RecalculateStats
  ;[1 1 1] Call after
  ; -Level UP
  ; -Learning new  Attribute  level
  ; -Equiped weapon changes
  (CallFunction|SetMaxHpMpSp)
  (CallFunction|SetRegen)
  (CallFunction|SetDamage))

(event EventBeginPlay
  (CallFunction|SetMaxHpMpSp)
  (CallFunction|SetRegen)
  (CallFunction|SetDamage))

(event EventTick
  (params (DeltaSeconds :type Float%20%28single-precision%29)))

(event EventGetHit
  (params (PhysicalDamage :type Float%20%28double-precision%29) (MagicalDamage :type Float%20%28double-precision%29))
  (bind _returnvalue (Components|GetOwner))
  (CallFunction|ReceiveWeaponDamage PhysicalDamage MagicalDamage)
  ;[1 0 0.01504] TODO call StartRegen  event
  (Class|BPICombatAttributes|StartRegen(Message) _returnvalue)
  ;[1 1 1] Check whether character should die
  (if (<= (Variables|Actor'sbasicstats|GetCurrentHp) 0.0)
    (CallFunction|TurnonRagDoll)
    ;[1 1 1] Turn's off - Cylinder collision of a dead body
    (bind _collision (Class|BPICharacterBase|GetCollisionCyllinder(Message) _returnvalue))
    (Collision|SetCollisionProfileName _collision "NoCollision" true :!class /Script/Engine.PrimitiveComponent)
    (Variables|Default|SetIsDead true)))

(fn RMBHitAnActor
  (params (EnemyTarget :type BPI%20Combat%20Attributes%20Interface))
  (Default|GetHit EnemyTarget (Variables|RMBOffenceStats|GetRMB_PhysicalDamage) (Variables|RMBOffenceStats|GetRMB_MagicalDamage)))

(fn LMBHitAnActor
  (params (EnemyTarget :type BPI%20Combat%20Attributes%20Interface))
  (Default|GetHit EnemyTarget (Variables|LMBOffenceStats|GetLMB_PhysicalDamage) (Variables|LMBOffenceStats|GetLMB_MagicalDamage)))

(fn GainExp
  (params (Quest%20or%20enemy%20Level :type Byte) (EXP%20To%20be%20gained :type Float%20%28double-precision%29))
  ;[1 1 1] Is the Player's lv greater than enemy's lv
  (if (> (Variables|Actor'sStats|GetActor's%20level) Quest%20or%20enemy%20Level)
    ;[1 1 1] How much greater is the player's lv than killed enemy's level
    (if (== (- (Variables|Actor'sStats|GetActor's%20level) 1) Quest%20or%20enemy%20Level) ; is greater by 1?
      (LocalVariables|SetExp%20Gain%20Rate 0.8)
      (elif (== (- (Variables|Actor'sStats|GetActor's%20level) 2) Quest%20or%20enemy%20Level) ; is greater by 2?
        (LocalVariables|SetExp%20Gain%20Rate 0.6)
        (elif (== (- (Variables|Actor'sStats|GetActor's%20level) 3) Quest%20or%20enemy%20Level) ; is greater by 3?
          (LocalVariables|SetExp%20Gain%20Rate 0.4)
          (elif (== (- (Variables|Actor'sStats|GetActor's%20level) 4) Quest%20or%20enemy%20Level) ; is greater by 4?
            (LocalVariables|SetExp%20Gain%20Rate 0.2)
            (else
              (LocalVariables|SetExp%20Gain%20Rate 0.0))))))
    (else
      (LocalVariables|SetExp%20Gain%20Rate 1.0)))
  ;[1 1 1] Grant player the exp
  (bind _output_get (Variables|Actor'sStats|SetActor's%20experience (+ (Variables|Actor'sStats|GetActor's%20experience) (* (LocalVariables|GetExp%20Gain%20Rate) EXP%20To%20be%20gained))))
  ;[1 1 1] Check if Player should lv up
  (if (> _output_get 1e+03)
    ;[1 1 1] Level++
    (Variables|Actor'sStats|SetActor's%20level (+ (Variables|Actor'sStats|GetActor's%20level) 1))
    ;[1 1 1] add Overboard exp to Player's Exp
    (Variables|Actor'sStats|SetActor's%20experience (- _output_get 1e+03))))

(fn ReceiveWeaponDamage
  (params (PhysicalDamage :type Float%20%28double-precision%29) (MagicalDamage :type Float%20%28double-precision%29))
  (bind _returnvalue (* PhysicalDamage 0.1))
  (bind _returnvalue_2 (* MagicalDamage 0.1))
  (bind _armour (Variables|DefenceStats|GetArmour))
  (bind _magicresistance (Variables|DefenceStats|GetMagicResistance))
  (bind _returnvalue_3 (- PhysicalDamage _armour))
  (bind _returnvalue_4 (+ _returnvalue _returnvalue_2))
  (bind _returnvalue_5 (- _magicresistance MagicalDamage))
  (bind _returnvalue_6 (Math|Float|Min(Float) _returnvalue_5 0.0))
  (bind _returnvalue_7 (Math|Float|Min(Float) _returnvalue_3 0.0))
  (bind _returnvalue_8 (+ _returnvalue_7 _returnvalue_6))
  (if (> _returnvalue_8 _returnvalue_4)
    ;[1 1 1] Deals normal damage ammount
    (Variables|Actor'sbasicstats|SetCurrentHp (- (Variables|Actor'sbasicstats|GetCurrentHp) _returnvalue_8))
    (else
      ;[1 1 1] Deals minimal damage ammount
      (Variables|Actor'sbasicstats|SetCurrentHp (- (Variables|Actor'sbasicstats|GetCurrentHp) _returnvalue_4)))))

(fn TurnonRagDoll
  (bind _returnvalue (Components|GetOwner))
  (bind _skeletalmeshcomponent (Class|BPICharacterBase|GetSkeletalMeshComponent(Message) _returnvalue))
  (bind _charactermovementcomponent (Class|BPICharacterBase|GetCharacterMovementComponent(Message) _returnvalue))
  (Physics|SetSimulatePhysics _skeletalmeshcomponent true)
  (Pawn|Components|CharacterMovement|DisableMovement _charactermovementcomponent))

(fn TurnOffRagDoll
  (bind _returnvalue (Components|GetOwner))
  (bind _skeletalmeshcomponent (Class|BPICharacterBase|GetSkeletalMeshComponent(Message) _returnvalue))
  (bind _charactermovementcomponent (Class|BPICharacterBase|GetCharacterMovementComponent(Message) _returnvalue))
  (Physics|SetSimulatePhysics _skeletalmeshcomponent false)
  ;[1 0 0] Test This to Enable movement component
  (Pawn|Components|CharacterMovement|SetMovementMode _charactermovementcomponent "MOVE_Walking" 0))

(fn SetMaxHpMpSp
  (bind _actor_s_level (Variables|Actor'sStats|GetActor's%20level))
  (bind _returnvalue (Math|Conversions|ToFloat(Byte) _actor_s_level))
  (bind _returnvalue_2 (* _returnvalue 5.0))
  (bind _output_get (Variables|Actor'sbasicstats|SetMaxHp (Math|Float|Max(Float) (* _returnvalue_2 (Math|Float|Max(Float) (/ (Math|Conversions|ToFloat(Byte) (Variables|Actor'sBasicStats|GetPhysique)) 1e+01) 1.0)) 1e+01)))
  (bind _output_get_2 (Variables|Actor'sbasicstats|SetMaxMp (Math|Float|Max(Float) (* _returnvalue_2 (Math|Float|Max(Float) (/ (Math|Conversions|ToFloat(Byte) (Variables|Actor'sBasicStats|GetWill)) 1e+01) 1.0)) 1e+01)))
  (bind _output_get_3 (Variables|Actor'sbasicstats|SetMaxSp (Math|Float|Max(Float) (* _returnvalue_2 (Math|Float|Max(Float) (/ (Math|Conversions|ToFloat(Byte) (Variables|Actor'sBasicStats|GetEndurance)) 1e+01) 1.0)) 1e+01)))
  ;[1 1 1] Sets current  hp  to match
  (Variables|Actor'sbasicstats|SetCurrentHp _output_get)
  (Variables|Actor'sbasicstats|SetCurrentMp _output_get_2)
  (Variables|Actor'sbasicstats|SetCurrentSp _output_get_3))

(fn SetRegen
  (bind _actor_s_level (Variables|Actor'sStats|GetActor's%20level))
  (bind _returnvalue (Math|Conversions|ToFloat(Byte) _actor_s_level))
  (bind _returnvalue_2 (* _returnvalue 0.5))
  ;[1 1 1] How much  of that  stat will be regenerated per every 5  secs
  (Variables|Actor'sBasicStats|SetHpRegen (* _returnvalue_2 (Math|Float|Max(Float) (/ (Math|Conversions|ToFloat(Byte) (Variables|Actor'sBasicStats|GetWoundClotting)) 2e+01) 1.0)))
  (Variables|Actor'sBasicStats|SetMpRegen (* _returnvalue_2 (Math|Float|Max(Float) (/ (Math|Conversions|ToFloat(Byte) (Variables|Actor'sBasicStats|GetMindPeace)) 1e+01) 1.0)))
  (Variables|Actor'sBasicStats|SetSpRegen (* _returnvalue_2 (Math|Float|Max(Float) (/ (Math|Conversions|ToFloat(Byte) (Variables|Actor'sBasicStats|GetResting)) 1e+01) 1.0))))

(fn SetDamage
  (bind _rmb (Class|BPICharacterBase|GetEquippedWeapon(Message) (Components|GetOwner)))
  (switch Utilities|FlowControl|Switch|SwitchonE_WeaponType (.WeaponType (Utilities|Struct|BreakS_WeaponInfo _rmb))))