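; Player controller Blueprint that opens the game's full UI screens: inventory, container, wait and game menu.
; Each open event creates its widget and adds it to the viewport only while the CanOpen flag is set, then clears that flag to block further screens.
; AllowOpenUI resumes cloth simulation on the player character's mesh, then sets CanOpen from its State input after a short anti-spam delay.
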(event EventBeginPlay)

(event EventTick
  (params (DeltaSeconds :type Float%20%28single-precision%29)))

(event EventOpenContainerUI
  (if (Variables|Default|GetCanOpen)
    (Variables|Default|SetCanOpen false)
    (bind _returnvalue (UserInterface|CreateWidget "/Game/_main/BP-Folder/Widgets/W_Container.W_Container_C" self))
    (UserInterface|Viewport|AddtoViewport _returnvalue 0)))

(event EventOpenInventoryUI
  (if (Variables|Default|GetCanOpen)
    (Variables|Default|SetCanOpen false)
    (bind _returnvalue (UserInterface|CreateWidget "/Game/_main/BP-Folder/Widgets/W_UI_2.W_UI_2_C" self))
    (UserInterface|Viewport|AddtoViewport _returnvalue 0)))

(event EventAllowOpenUI
  (params (State :type Boolean))
  ;[1 1 1] Allow the cloth sim. after quiting ui
  (Class|SkeletalMeshComponent|ResumeClothingSimulation (Variables|/Script/Engine.Character|GetMesh (Game|GetPlayerCharacter 0)))
  (Utilities|FlowControl|Delay 0.2) ; Just to prevent spam opening UIs
  ;[1 1 1] Allow to open new ui
  (Variables|Default|SetCanOpen State))

(event EventOpenWaitUI
  (if (Variables|Default|GetCanOpen)
    (Variables|Default|SetCanOpen false)
    (bind _returnvalue (UserInterface|CreateWidget "/Game/_main/BP-Folder/Widgets/Wait/W_WaitUI.W_WaitUI_C" self))
    (UserInterface|Viewport|AddtoViewport _returnvalue 0)))

(event EventOpenGameMenuUI
  (if (Variables|Default|GetCanOpen)
    (Variables|Default|SetCanOpen false)
    (bind _returnvalue (UserInterface|CreateWidget "/Game/_main/BP-Folder/Widgets/GameMenuUI/W_GameMenuUI.W_GameMenuUI_C" self))
    (UserInterface|Viewport|AddtoViewport _returnvalue 0)))

(fn ConstructionScript)