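; Base humanoid AI Blueprint that advances an NPC's wealth and rest state over game time.
; On BeginPlay it calls the parent, then starts a timeline whose event track is noted to fire every 360 seconds, or two in-game hours.
; Each event increments CurrentWealthState and lowers RestLevel on the BPCBasicAttributes component, a rest mechanic marked as tentative for NPCs.
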(event EventBeginPlay
  (bind _bpc_basicattributes (Variables|Default|GetBPC_BasicAttributes))
  (|CallParentFunction)
  (Timeline|Timeline_1 PlayFromStart ; Currently ticks every 360 secs  which is 2h of in-game time
    (:EventTrack%20-%20Tick
      (Variables|Default|SetcurrentWealthState (+ (Variables|Default|GetcurrentWealthState) 1))
      ;[1 1 1] Still not sure if  I really want  to use this  mechanics on NPC
      (Variables|/Game/_main/BP-Folder/BPs_Base/BPC_BasicAttributes.BPC_BasicAttributes_C|SetrestLevel _bpc_basicattributes (- (Variables|/Game/_main/BP-Folder/BPs_Base/BPC_BasicAttributes.BPC_BasicAttributes_C|GetrestLevel _bpc_basicattributes) 10)))))

(event Collision|EventActorBeginOverlap
  (params (OtherActor :type Actor%20Object%20Reference))
  (|CallParentFunction OtherActor) ; This node is disabled and will not be called.\nDrag off pins to build functionality.
)

(event EventTick
  (params (DeltaSeconds :type Float%20%28single-precision%29))
  (|CallParentFunction DeltaSeconds) ; This node is disabled and will not be called.\nDrag off pins to build functionality.
)

(fn ConstructionScript
  (|CallParentFunction))